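; Base vehicle pawn Blueprint whose graphs currently run no logic: its overlap, tick and construction script are empty.
; An unconnected tip-over check compares mesh roll and pitch to a threshold, rechecks after a delay, then calls SoftReset if still tipped, gated by ToggleAutomaticSoftReset.
; A second unconnected fragment applies a mass-scaled vertical impulse with a fixed X push to the mesh.
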(event `self.ReceiveTick`
  (params (DeltaSeconds :type "Float (single-precision)")))

(event `InputAction|Jump`
  (params (Key :type "Key Structure")))

(fn `UserConstructionScript`)